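; Interactable door that swings away from or toward a side chosen by the player's facing, cycling through cracked, fully open and closed.
; Tick polls the player character's interact flag and hit actor, using a dot product to pick the side and interpolating the yaw per state.
; A timer ends each interaction and advances the state enum.
; Leaving the box at certain facings briefly re-flags interaction and nudges the door toward closed, without changing state.
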(event OnComponentEndOverlap(Box)
  (params (OverlappedComponent :type Primitive%20Component%20Object%20Reference) (OtherActor :type Actor%20Object%20Reference) (OtherComp :type Primitive%20Component%20Object%20Reference) (OtherBodyIndex :type Integer))
  (bind _returnvalue (Game|GetPlayerCharacter 0))
  (bind _returnvalue_2 (Transformation|GetActorForwardVector _returnvalue))
  (if (and (== OtherActor _returnvalue) (Math|Boolean|NORBoolean (>= (.y _returnvalue_2) 0.7) (<= (.y _returnvalue_2) -0.7)))
    (Utilities|FlowControl|Delay 0.5)
    (Variables|Default|SetbIsInteractingWithDoor? true)
    (CallFunction|DoorRotation 0.0)
    (Utilities|FlowControl|Delay 1.4)
    (Variables|Default|SetbIsInteractingWithDoor? false)))

(event Custom|DoorRotation
  (params (Set%20Rotation :type Float%20%28double-precision%29))
  (Transformation|SetRelativeRotation (Variables|Default|GetDoor) (Math|Rotator|MakeRotator 0.0 0.0 (Math|Interpolation|FInterpTo (.Yaw (Math|Rotator|BreakRotator (Variables|/Script/Engine.SceneComponent|GetRelativeRotation (Variables|Default|GetDoor)))) Set%20Rotation (Utilities|Time|GetWorldDeltaSeconds) (Variables|Default|GetInterp%20Speed))) false false))

(event Custom|HandleDoor
  ;[0 0.002792 0.15 0.5] Door Handling - Rotate the door based on the current set door enum state.
  (switch Utilities|FlowControl|Switch|SwitchonE_DoorStates (Variables|Default|GetEDoorStates)
    (:NewEnumerator0
      (CallFunction|DoorRotation (* 15.0 (Variables|Default|GetDoor%20Open%20Side))))
    (:NewEnumerator1
      (CallFunction|DoorRotation (* (Variables|Default|GetDoor%20Open%20Angle) (Variables|Default|GetDoor%20Open%20Side))))
    (:NewEnumerator2
      (CallFunction|DoorRotation 0.0))))

(event Custom|isInteractingWithDoor
  (params (Player :type BP%20Third%20Person%20Character%20Object%20Reference))
  ;[0.00223 0 0.15 0.5] Door Interaction Mathematics
  (if (> (Math|Vector|DotProduct (Transformation|GetActorForwardVector Player) (Math|Vector|GetForwardVector (Variables|Default|GetDoorOpenLocation))) 0.0)
    (Variables|Default|SetDoor%20Open%20Side 1.0)
    (else
      (Variables|Default|SetDoor%20Open%20Side -1.0)))
  (Variables|Default|SetbIsInteractingWithDoor? true)
  (Utilities|Time|SetTimerbyEvent (delegate Custom|CustomEvent) (Variables|Default|GetDoor%20Sound%20Time)))

(event Custom|CustomEvent
  ;[0.00223 0 0.15 0.5] Door Interaction Mathematics
  (Variables|Default|SetbIsInteractingWithDoor? false)
  (switch Utilities|FlowControl|Switch|SwitchonE_DoorStates (Variables|Default|GetEDoorStates)
    (:NewEnumerator0
      (Variables|Default|SetEDoorStates "NewEnumerator1"))
    (:NewEnumerator1
      (Variables|Default|SetEDoorStates "NewEnumerator2"))
    (:NewEnumerator2
      (Variables|Default|SetEDoorStates "NewEnumerator0"))))

(event EventBeginPlay
  (bind _asbp_third_person_character (Utilities|Casting|CastToBP_ThirdPersonCharacter (Game|GetPlayerCharacter 0)))
  (Variables|Default|SetCharacterReference _asbp_third_person_character))

(event EventTick
  (params (DeltaSeconds :type Float%20%28single-precision%29))
  (bind _characterreference (Variables|Default|GetCharacterReference))
  (if (and (Variables|/Game/ThirdPerson/Blueprints/BP_ThirdPersonCharacter.BP_ThirdPersonCharacter_C|GetisInteracting? _characterreference) (== (Variables|/Game/ThirdPerson/Blueprints/BP_ThirdPersonCharacter.BP_ThirdPersonCharacter_C|GetHit%20Actor _characterreference) self))
    (if (Variables|Default|GetbIsInteractingWithDoor?)
      (CallFunction|HandleDoor)
      (else
        (CallFunction|IsInteractingwithDoor (Variables|Default|GetCharacterReference))))))

(fn ConstructionScript)

(fn Interactable
  (params (Interactor :type BP%20Third%20Person%20Character%20Object%20Reference))
  (return))