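; BP_KeyHintDecal is a decal actor that stays hidden until the player character's hint flag turns on.
; On BeginPlay it caches the BP_ThirdPersonCharacter player reference and hides its decal.
; Tick polls the character's HintVisible flag and uses a DoOnce to reveal the decal a single time, with no logic to hide it again.
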(event EventBeginPlay
  (bind _asbp_third_person_character (Utilities|Casting|CastToBP_ThirdPersonCharacter (Game|GetPlayerCharacter 0)))
  (Variables|Default|SetBP%20Char%20Ref _asbp_third_person_character)
  (bind _output_get (Variables|Default|SetVisible? false))
  (Rendering|SetVisibility (Variables|Default|GetDECAL) _output_get false))

(event EventTick
  (params (DeltaSeconds :type Float%20%28single-precision%29))
  (if (Variables|/Game/ThirdPerson/Blueprints/BP_ThirdPersonCharacter.BP_ThirdPersonCharacter_C|GetHintVisible? (Variables|Default|GetBP%20Char%20Ref))
    (Utilities|FlowControl|DoOnce false
      (:Completed
        (bind _output_get (Variables|Default|SetVisible? true))
        (Rendering|SetVisibility (Variables|Default|GetDECAL) _output_get false)))))

(fn ConstructionScript)