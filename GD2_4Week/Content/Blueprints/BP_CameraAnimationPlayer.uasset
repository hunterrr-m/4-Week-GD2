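; BP_CameraAnimationPlayer is a temporary view-target actor that plays a camera animation for the first player.
; PlayCameraAnimation starts the animation through the EngineCamerasSubsystem and blends player 0's view to this actor.
; EndCameraAnimation blends the view back to the player character, waits out the one-second blend, then destroys the actor.
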(event Custom|PlayCameraAnimation
  (bind _returnvalue (Game|GetPlayerController 0))
  (Class|EngineCamerasSubsystem|PlayCameraAnimation (Subsystems|GetEngineCamerasSubsystem) _returnvalue)
  (Game|Player|SetViewTargetwithBlend _returnvalue self 1.0 "VTBlend_Linear" 0.0 false))

(event Custom|EndCameraAnimation
  (Game|Player|SetViewTargetwithBlend (Game|GetPlayerController 0) (Game|GetPlayerCharacter 0) 1.0 "VTBlend_Linear" 0.0 false)
  (Utilities|FlowControl|Delay 1.0)
  (Actor|DestroyActor))

(fn ConstructionScript)