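; BP_Endtable is an interactable end table with a drawer that toggles open and closed.
; Each interaction passes through a FlipFlop that alternately plays and reverses the DrawerMovement timeline.
; The timeline's OpenClose alpha interpolates the drawer's relative location between CloseLocation and OpenLocation.
; When KeyEnabled is set, the referenced base item's mesh receives the same relative location, moving it with the drawer.
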(event Custom|Open%20and%20Close
  (Utilities|FlowControl|FlipFlop
    (:A
      (bind _openclose (Timeline|DrawerMovement Play)
        (:Update
          (Transformation|SetRelativeLocation (Variables|Default|GetDrawer) (Math|Vector|Lerp(Vector) (Variables|Default|GetClose%20Location) (Variables|Default|GetOpen%20Location) _openclose) false false)
          (if (Variables|Default|GetKeyEnabled?)
            (Transformation|SetRelativeLocation (Variables|/Game/ThirdPerson/Blueprints/BP_BaseItem.BP_BaseItem_C|GetStaticMesh (Variables|Default|GetBP%20BaseItem%20Ref)) (Math|Vector|Lerp(Vector) (Variables|Default|GetClose%20Location) (Variables|Default|GetOpen%20Location) _openclose) false false)))))
    (:B
      (Timeline|DrawerMovement Reverse))))

(event EventInteractable
  (params (Interactor :type BP%20Third%20Person%20Character%20Object%20Reference))
  (CallFunction|OpenandClose))

(fn ConstructionScript)